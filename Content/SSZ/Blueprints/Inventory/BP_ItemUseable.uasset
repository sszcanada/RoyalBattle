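; BP_ItemUseable is a usable inventory item whose mesh and data come from the item database, selected by ItemNumber.
; SetupMesh sets the root's static mesh and copies the entry's name, description, effect and effect arguments into its variables.
; It runs in both the construction script and BeginPlay, while applying the effect is not handled here.
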(event `self.ReceiveBeginPlay`
  (`self.SetupMesh`))

(fn `SetupMesh`
  (bind _struct_itemdatabase_itemdatabase (break `/Game/SSZ/Blueprints/Inventory/Components/Struct_ItemDatabase` (make `/Game/SSZ/Blueprints/Inventory/Components/Struct_ItemDatabase` _)))
  (bind (_output_itemmesh_static _output_itemname _output_itemdescription _output_itemeffect _output_effectarguments) (break `/Game/SSZ/Blueprints/Inventory/Components/Struct_ItemSingle` (`|GetArrayItem` _struct_itemdatabase_itemdatabase (`self.ItemNumber`))))
  (`StaticMeshComponent.SetStaticMesh` (`self.Root`) _output_itemmesh_static)
  (set `self.ItemName` _output_itemname)
  (set `self.ItemDescription` _output_itemdescription)
  (set `self.ItemEffect` _output_itemeffect)
  (set `self.EffectArguments` _output_effectarguments))

(fn `UserConstructionScript`
  (`self.SetupMesh`))