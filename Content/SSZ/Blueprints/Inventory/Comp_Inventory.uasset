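; Inventory component that stores item number and amount pairs and persists them to an encrypted local file.
; AddToInventory loads the file, checks capacity, then appends the item and saves.
; SaveInventory schema-encodes and encrypts each row with a hardcoded key, overwriting the file at a fixed absolute path.
; LoadInventory decrypts rows and appends them without clearing the array, filling both number and amount from the first field.
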(fn `AddToInventory`
  (params (ItemToAdd :type Integer) (AmountToAdd :type Integer))
  (bind _inventory (`self.Inventory`))
  (bind _returnvalue (`KismetArrayLibrary.Array_LastIndex` _inventory))
  (`self.LoadInventory`)
  (if (and (>= (+ _returnvalue 1) (`self.MaxInventorySize`)) (!= _returnvalue 0))
    (`KismetSystemLibrary.PrintString` "No Space Left")
    (else
      (`KismetArrayLibrary.Array_Add` _inventory (make `/Game/SSZ/Blueprints/Inventory/Components/Struct_InventorySingle` ItemToAdd AmountToAdd))
      (`self.SaveInventory`))))

(fn `LoadInventory`
  (bind (_report _success _arrayinfile) (`SSZFileFunctions.LoadStringArrayFromFile` "C:\\RoyalBattle\\Content\\SSZ\\Extra" "Inventory.ssz"))
  (if _success
    (for _array_element _arrayinfile
      (bind _returnvalue (`Encryption.Decrypt` _array_element "r4u7x!A%C*F-JaNdRgUkXp2s5v8y/B?E"))
      (bind _schemaarray (`/SSZCode/Components/BP_Macros_Core.SchemaRowDecoder` _returnvalue))
      (`KismetArrayLibrary.Array_Add` (`self.Inventory`) (make `/Game/SSZ/Blueprints/Inventory/Components/Struct_InventorySingle` (`KismetStringLibrary.Conv_StringToInt` (`|GetArrayItem` _schemaarray)) (`KismetStringLibrary.Conv_StringToInt` (`|GetArrayItem` _schemaarray)))))
    (else
      (`SSZFileFunctions.SaveStringArrayToFile` "C:\\RoyalBattle\\Content\\SSZ\\Extra" "Inventory.ssz" (`self.ArrayStrings`)))))

(fn `SaveInventory`
  (locals (Empty :type "Array of String"))
  (set `self.ArrayStrings` (`local.Empty`))
  (for _array_element (`self.Inventory`)
    (bind _returnvalue (`Encryption.Encrypt` (`/SSZCode/Components/BP_Macros_Core.SchemaRowEncoder` (`|MakeArray` (`KismetStringLibrary.Conv_IntToString` (break `/Game/SSZ/Blueprints/Inventory/Components/Struct_InventorySingle` _array_element)) (`KismetStringLibrary.Conv_IntToString` (`.ItemAmount_4_ABF5CFCB43AC161D5D671CAD0D5D8D2B` (break `/Game/SSZ/Blueprints/Inventory/Components/Struct_InventorySingle` _array_element))))) "r4u7x!A%C*F-JaNdRgUkXp2s5v8y/B?E"))
    (`KismetArrayLibrary.Array_Add` (`self.ArrayStrings`) _returnvalue))
  (`SSZFileFunctions.SaveStringArrayToFile` "C:\\RoyalBattle\\Content\\SSZ\\Extra" "Inventory.ssz" (`self.ArrayStrings`) true)
  (set `self.ArrayStrings` (`local.Empty`)))