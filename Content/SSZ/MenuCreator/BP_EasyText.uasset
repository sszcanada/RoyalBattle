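; BP_EasyText is a menu text actor combining Text3D and TextRender components with a scalable button mesh and a select component.
; The construction script applies the button mesh and scale, showing either a preview material or M_Alpha depending on visibility.
; Functions restyle the 3D or 2D text directly or from indexed text database entries, using helpers to convert alignments.
; The select-press event is an empty stub.
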(event `self.Comp_Select_Component.PressedSelect`
  (params (Pawn :type "/Game/AFCore/Blueprints/Pawn/BP_Pawn_Base Object Reference") (SourceActor :type "Actor Object Reference") (ImpactLocation :type "Vector Structure") (ImpactComponent :type "ActorComponent Object Reference")))

(fn `Change2DText`
  (params (Text :type Text) (HorizonalAlignment :type "EHorizTextAligment Enum" :default "EHTA_Center") (VerticalAlignment :type "EVerticalTextAligment Enum" :default "EVRTA_TextCenter") (Colour :type "LinearColor Structure") (TextScale :type "Float (double-precision)" :default 15.0) (ButtonScale :type "Vector Structure"))
  (bind _textrender (`self.TextRender`))
  (`TextRenderComponent.K2_SetText` _textrender Text)
  (`TextRenderComponent.SetHorizontalAlignment` _textrender HorizonalAlignment)
  (`TextRenderComponent.SetVerticalAlignment` _textrender VerticalAlignment)
  (`TextRenderComponent.SetTextRenderColor` _textrender (`KismetMathLibrary.Conv_LinearColorToColor` Colour))
  (`TextRenderComponent.SetWorldSize` _textrender TextScale)
  (bind _output_get (set `self.ButtonScale` ButtonScale))
  (`self.ChangeButtonScale` _output_get))

(fn `Change2DTextFromDatabase`
  (params (DatabaseIndex :type Integer))
  (bind (_struct_textdatabase_3dtextdatabase _struct_textdatabase_2dtextdatabase) (break `/Game/SSZ/MenuCreator/Struct_TextDatabase` (make `/Game/SSZ/MenuCreator/Struct_TextDatabase` _)))
  (bind (_output_text _output_buttonscale _output_horizonalalignment _output_verticalalignment _output_colour _output_scale) (break `/Game/SSZ/MenuCreator/SubComponents/Struct_TextSingle2D` (`|GetArrayItem` _struct_textdatabase_2dtextdatabase DatabaseIndex)))
  (`self.Change2DText` _output_text (select `/Game/SSZ/MenuCreator/SubComponents/Enum_AlignmentHelperHo` _output_horizonalalignment :`NewEnumerator0` "EHTA_Left" :`NewEnumerator1` "EHTA_Center" :`NewEnumerator2` "EHTA_Right" :!type "EHorizTextAligment Enum") (select `/Game/SSZ/MenuCreator/SubComponents/Enum_AlignmentHelperVe2` _output_verticalalignment :`NewEnumerator0` "EVRTA_TextTop" :`NewEnumerator1` "EVRTA_TextCenter" :`NewEnumerator2` "EVRTA_TextBottom" :`NewEnumerator4` "EVRTA_QuadTop" :!type "EVerticalTextAligment Enum") _output_colour _output_scale))

(fn `Change3DText`
  (params (Text :type Text) (Extrude :type "Float (double-precision)" :default 5.0) (Material :type "MaterialInterface Object Reference") (HorizonalAlignment :type "EText3DHorizontalTextAlignment Enum" :default "Center") (VerticalAlignment :type "EText3DVerticalTextAlignment Enum" :default "Center") (LineSpacing :type "Float (double-precision)") (WordSpacing :type "Float (double-precision)") (ButtonScale :type "Vector Structure" :default (1.0 1.0 0.0)))
  (bind _text3d (`self.Text3D`))
  (`Text3DComponent.SetText` _text3d Text)
  (`Text3DComponent.SetExtrude` _text3d Extrude)
  (`Text3DComponent.SetBackMaterial` _text3d Material)
  (`Text3DComponent.SetExtrudeMaterial` _text3d Material)
  (`Text3DComponent.SetBevelMaterial` _text3d Material)
  (`Text3DComponent.SetFrontMaterial` _text3d Material)
  (`Text3DComponent.SetHorizontalAlignment` _text3d HorizonalAlignment)
  (`Text3DComponent.SetVerticalAlignment` _text3d VerticalAlignment)
  (`Text3DComponent.SetLineSpacing` _text3d LineSpacing)
  (`Text3DComponent.SetWordSpacing` _text3d WordSpacing)
  (bind _output_get (set `self.ButtonScale` ButtonScale))
  (`self.ChangeButtonScale` _output_get))

(fn `Change3DTextFromDatabase`
  (params (DatabaseIndex :type Integer))
  (bind _struct_textdatabase_3dtextdatabase (break `/Game/SSZ/MenuCreator/Struct_TextDatabase` (make `/Game/SSZ/MenuCreator/Struct_TextDatabase` _)))
  (bind (_output_text _output_buttonscale _output_extrude _output_material _output_horizonalalignment _output_virticalalignment _output_linespcaing _output_wordspacing) (break `/Game/SSZ/MenuCreator/SubComponents/Struct_TextSingle3D` (`|GetArrayItem` _struct_textdatabase_3dtextdatabase DatabaseIndex)))
  (`self.Change3DText` _output_text _output_extrude _output_material (select `/Game/SSZ/MenuCreator/SubComponents/Enum_AlignmentHelperHo` _output_horizonalalignment :`NewEnumerator0` "Left" :`NewEnumerator1` "Center" :`NewEnumerator2` "Right" :!type "EText3DHorizontalTextAlignment Enum") (select `/Game/SSZ/MenuCreator/SubComponents/Enum_AlignmentHelperVe` _output_virticalalignment :`NewEnumerator0` "FirstLine" :`NewEnumerator1` "FirstLine" :`NewEnumerator2` "FirstLine" :`NewEnumerator4` "FirstLine" :!type "EText3DVerticalTextAlignment Enum") _output_linespcaing _output_wordspacing)
  (bind _output_get (set `self.ButtonScale` _output_buttonscale))
  (`self.ChangeButtonScale` _output_get))

(fn `ChangeButtonScale`
  (params (NewScale :type "Vector Structure"))
  (`SceneComponent.SetWorldScale3D` (`self.Mesh_Button_OuterBarrier`) NewScale))

(fn `UserConstructionScript`
  (bind _mesh_button_outerbarrier (`self.Mesh_Button_OuterBarrier`))
  (`StaticMeshComponent.SetStaticMesh` _mesh_button_outerbarrier (`self.ButtonMesh`))
  (`self.ChangeButtonScale` (`self.ButtonScale`))
  (if (`self.ButtonVisable`)
    (`PrimitiveComponent.SetMaterial` _mesh_button_outerbarrier 0 (`self.ButtonPreviewMaterial`))
    (else
      (`PrimitiveComponent.SetMaterial` _mesh_button_outerbarrier 0 "/Game/SSZ/MenuCreator/SubComponents/M_Alpha.M_Alpha"))))